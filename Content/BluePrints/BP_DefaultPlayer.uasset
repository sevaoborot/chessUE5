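; BP_DefaultPlayer is the player Blueprint for mouse-driven figure selection in what appears to be a turn-based board game.
; BeginPlay shows the cursor, and each left click calls DoLineTrace, which stores the actor hit under the cursor as CurrentFigure.
; With a valid CurrentFigure, the trace channel follows IsWhiteActiveRN and a valid hit prints a debug message; otherwise a third channel is used.
; An older camera-forward trace remains unconnected.
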(event EventBeginPlay
  (Variables|/Script/Engine.PlayerController|SetbShowMouseCursor (Game|GetPlayerController 0) true))

(event Collision|EventActorBeginOverlap
  (params (OtherActor :type Actor%20Object%20Reference)))

(event EventTick
  (params (DeltaSeconds :type Float%20%28single-precision%29)))

(event Input|MouseEvents|LeftMouseButton
  (params (Key :type Key%20Structure :default "None"))
  (bind _currentfigure (Variables|Default|GetcurrentFigure))
  (bind _returnvalue (Utilities|IsValid _currentfigure))
  (:Pressed
    (if _returnvalue
      (if (Variables|Default|GetisWhiteActiveRN)
        (CallFunction|DoLineTrace "TraceTypeQuery4")
        (else
          (CallFunction|DoLineTrace "TraceTypeQuery3")))
      (if _returnvalue
        (Development|PrintString "figure selected!"))
      (else
        (CallFunction|DoLineTrace "TraceTypeQuery5")))))

(fn ConstructionScript)

(fn DoLineTrace
  (params (Channel :type ETraceTypeQuery%20Enum :default "TraceTypeQuery1"))
  (Variables|Default|SetcurrentFigure (.HitActor (Collision|BreakHitResult (.HitResult (Game|Player|GetHitResultUnderCursorbyChannel (Game|GetPlayerController 0) Channel true)))))
  (return))