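; Chess board manager that tracks which figure occupies each cell and validates chosen moves.
; On BeginPlay it converts every BP_Figure's world location to cell coordinates and registers it through SetFigures.
; Move validation checks the chosen cell against the possible-movement list and deletes any occupying figure, without a colour check.
; A separate pawn check allows attack-only moves onto opposite-colour figures and normal moves onto empty cells.
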(event EventBeginPlay
  (bind _outactors (Actor|GetAllActorsOfClass "/Game/BluePrints/current/BP_Figure.BP_Figure_C"))
  (for _array_element _outactors
    ;[1 1 1] setting figures
    (Utilities|IsValid _array_element
      (:Is%20Valid
        (bind (_x _y) (Class|ChessMap|RealLocationtoCells (Transformation|GetActorLocation _array_element)))
        (Class|ChessMap|SetFigures _x _y _array_element))
      (:Is%20Not%20Valid
        (Development|PrintString "obj i not valid")))))

(event Collision|EventActorBeginOverlap
  (params (OtherActor :type Actor%20Object%20Reference)))

(event EventTick
  (params (DeltaSeconds :type Float%20%28single-precision%29)))

(fn ConstructionScript)

(fn FIsChosenCellsValid
  (params (currentCell :type Actor%20Object%20Reference) (possibleFigureMovements :type Array%20of%20ST%20Possible%20Figure%20Movements%20Structures))
  (if (Utilities|IsValid currentCell)
    (bind (_x _y) (Class|ChessMap|RealLocationtoCells (Transformation|GetActorLocation currentCell)))
    (if (Utilities|Array|ContainsItem possibleFigureMovements (Utilities|Struct|MakeST_possibleFigureMovements _x _y))
      (bind _returnvalue (Class|ChessMap|IsCellTaken _x _y))
      (if _returnvalue
        (bind _returnvalue_2 (Class|ChessMap|GetFigure _x _y))
        (Class|Figure|DeleteFigure _returnvalue_2 self)
        (return true)
        (else
          (Variables|Default|SetisChosenCellValid true)))
      (else
        (Development|PrintString "not into possibles range" true true "(R=1.000000,G=0.000000,B=0.997332,A=1.000000)")
        (bind _output_get (Variables|Default|SetisChosenCellValid false))
        (return _output_get)))))

(fn SettingAllFigures)

(fn FIsChosenCellValidforPawnAttack
  (params (x :type Integer) (y :type Integer) (isAttackOnly :type Boolean) (IsCosenFigureWhite :type Boolean))
  (Development|PrintString (Utilities|String|Append (Utilities|String|ToString(Integer) x) (Utilities|String|ToString(Integer) y)) true true "(R=0.000000,G=0.660000,B=1.000000,A=1.000000)" 1e+01)
  (bind _returnvalue (Class|ChessMap|IsCellTaken x y))
  (if _returnvalue
    (if isAttackOnly
      (bind _returnvalue_2 (Class|ChessMap|GetFigure x y))
      (if (== (Variables|/Script/NewChess.Figure|GetIsWhite _returnvalue_2) IsCosenFigureWhite)
        (Development|PrintString "same color" true true "(R=1.000000,G=0.000000,B=0.062871,A=1.000000)" 1e+01)
        (return false)
        (else
          (Development|PrintString "not same color" true true "(R=1.000000,G=0.000000,B=0.063010,A=1.000000)" 1e+01)
          (return true)))
      (else
        (return false)))
    (else
      (Development|PrintString "empty")
      (if isAttackOnly
        (return false)
        (else
          (return true))))))