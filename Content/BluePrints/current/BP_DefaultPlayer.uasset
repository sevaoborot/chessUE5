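; BP_DefaultPlayer is the player Blueprint for a chess game, handling mouse-driven piece and cell selection with alternating white and black turns.
; BeginPlay shows the cursor and caches the BP_ChessMap actor.
; Left click first picks a BP_Figure via a side-specific cursor trace channel and computes its moves.
; The next click traces for a cell, which ChessMap validates before clearing positions and switching turns.
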(event EventBeginPlay
  (Variables|/Script/Engine.PlayerController|SetbShowMouseCursor (Game|GetPlayerController 0) true)
  ;[1 1 1] ref to BP_ChessMap
  (bind _outactors (Actor|GetAllActorsOfClass "/Game/BluePrints/current/BP_ChessMap.BP_ChessMap_C"))
  (Variables|Refs|SetchessMap (Utilities|Array|Get(acopy) _outactors)))

(event Collision|EventActorBeginOverlap
  (params (OtherActor :type Actor%20Object%20Reference)))

(event EventTick
  (params (DeltaSeconds :type Float%20%28single-precision%29)))

(event Input|MouseEvents|LeftMouseButton
  (params (Key :type Key%20Structure))
  (bind _current (Variables|Refs|Getcurrent))
  (:Pressed
    (if (Variables|Bools|GetisFigureChosen)
      ;[1 1 1] For choosing sell (if figure is chosen)
      (if (Utilities|IsValid _current)
        (CallFunction|DoLineTrace "TraceTypeQuery5")
        (bind _isvalid (Default|FIsChosenCellValid (Variables|Refs|GetchessMap) _current (Variables|/Script/NewChess.Figure|GetIsWhite (Variables|Refs|GetchosenFigure)) (Variables|/Game/BluePrints/current/BP_Figure.BP_Figure_C|GetpossibleMoves (Variables|Refs|GetchosenFigure))))
        (if _isvalid
          (Development|PrintText "Cell is chosen")
          (Variables|Bools|SetisFigureChosen false)
          (Default|ClearPositions (Variables|Refs|GetchosenFigure))
          (if (Variables|Bools|GetisWhiteActiveRN)
            (Variables|Bools|SetisWhiteActiveRN false)
            (else
              (Variables|Bools|SetisWhiteActiveRN true)))
          (else
            (Development|PrintText "cell is occupied by another figure")))
        (else
          (Development|PrintText "figure is not chosen")))
      (else
        ;[1 1 1] For choosing figure
        (if (Variables|Bools|GetisWhiteActiveRN)
          (CallFunction|DoLineTrace "TraceTypeQuery4")
          (else
            (CallFunction|DoLineTrace "TraceTypeQuery3")))
        (if (Utilities|IsValid (Variables|Refs|Getcurrent))
          (bind _asbp_figure (Utilities|Casting|CastToBP_Figure (Variables|Refs|Getcurrent))
            (:then
              (bind _output_get (Variables|Refs|SetchosenFigure _asbp_figure))
              (Variables|Bools|SetisFigureChosen true)
              (Default|FindLogicalPositions _output_get 7))
            (:CastFailed
              (Development|PrintText "Cast failed"))))))))

(fn ConstructionScript)

(fn DoLineTrace
  (params (Channel :type ETraceTypeQuery%20Enum :default "TraceTypeQuery1"))
  (Variables|Refs|Setcurrent (.HitActor (Collision|BreakHitResult (.HitResult (Game|Player|GetHitResultUnderCursorbyChannel (Game|GetPlayerController 0) Channel true)))))
  (return))