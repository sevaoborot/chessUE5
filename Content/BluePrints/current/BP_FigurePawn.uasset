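; BP_FigurePawn is the pawn piece of a chess game, overriding the parent figure's move search.
; FindLogicalPositions offsets the current grid square by each Movement direction once, ignoring MaxMoves and flipping X for non-white pieces.
; Squares inside the 8x8 board are added to PossibleMoves, with no occupancy check here.
; The parent implementation is left unwired, and the event graph holds only disabled default events.
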(event EventBeginPlay
  (|CallParentFunction) ; This node is disabled and will not be called.\nDrag off pins to build functionality.
)

(event Collision|EventActorBeginOverlap
  (params (OtherActor :type Actor%20Object%20Reference))
  (|CallParentFunction OtherActor) ; This node is disabled and will not be called.\nDrag off pins to build functionality.
)

(event EventTick
  (params (DeltaSeconds :type Float%20%28single-precision%29))
  (|CallParentFunction DeltaSeconds) ; This node is disabled and will not be called.\nDrag off pins to build functionality.
)

(fn ConstructionScript
  (|CallParentFunction))

(fn FindLogicalPositions
  (params (maxMoves :type Integer))
  (bind (_x _y) (Class|Figure|CountGridPos))
  (for _array_element (Variables|Default|GetMovement)
    (LocalVariables|SetlocalX _x)
    (LocalVariables|SetlocalY _y)
    (if (Variables|Default|GetIsWhite)
      (LocalVariables|SetlocalX (+ (Math|Float|Truncate (.X (Class|KismetMathLibrary|BreakVector3f (.Direction (Utilities|Struct|BreakST_Movement _array_element))))) (LocalVariables|GetlocalX)))
      (else
        (LocalVariables|SetlocalX (- (LocalVariables|GetlocalX) (Math|Float|Truncate (.X (Class|KismetMathLibrary|BreakVector3f (.Direction (Utilities|Struct|BreakST_Movement _array_element)))))))))
    (LocalVariables|SetlocalY (+ (Math|Float|Truncate (.Y (Class|KismetMathLibrary|BreakVector3f (.Direction (Utilities|Struct|BreakST_Movement _array_element))))) (LocalVariables|GetlocalY)))
    (if (not (or (or (>= (LocalVariables|GetlocalX) 8) (>= (LocalVariables|GetlocalY) 8)) (or (<= (LocalVariables|GetlocalX) -1) (<= (LocalVariables|GetlocalY) -1))))
      (Utilities|Array|Add (Variables|Default|GetpossibleMoves) (Utilities|Struct|MakeST_possibleFigureMovements (LocalVariables|GetlocalX) (LocalVariables|GetlocalY))))))