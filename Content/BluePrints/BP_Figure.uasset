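; BP_Figure is a chess piece actor that registers itself on a chess map.
; Its construction script converts the Cylinder component's world X and Y into grid indices, dividing by 100 and truncating, then passes them with itself to ChessMapRef's SetFigures.
; MoveToNewPos is an empty stub, and the event graph has no active logic.
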(event EventBeginPlay)

(event Collision|EventActorBeginOverlap
  (params (OtherActor :type Actor%20Object%20Reference)))

(event EventTick
  (params (DeltaSeconds :type Float%20%28single-precision%29)))

(fn ConstructionScript
  (bind _cylinder (Variables|Default|GetCylinder))
  (bind _returnvalue (Transformation|GetWorldLocation _cylinder))
  (bind (_x _y) (Class|KismetMathLibrary|BreakVector3f _returnvalue))
  (bind _output_get (LocalVariables|SetlocalX (Math|Float|Truncate (/ _x 1e+02))))
  (bind _output_get_2 (LocalVariables|SetlocalY (Math|Float|Truncate (/ _y 1e+02))))
  (Class|ChessMap|SetFigures (Variables|Default|GetchessMapRef) _output_get _output_get_2 self))

(fn MovetoNewPos)